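; Short-lived range attack actor that damages enemies overlapping it and shows a fading point light.
; Tick lowers the light intensity by a fixed step each frame, independent of delta time, and destroys the actor once its accumulated lifetime reaches DestroyTime.
; On overlap, if the instigator is a Character, it calls GetDamage on the BaseEnemy with damage and stun values, flagged as a downward super attack.
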(event `self.ReceiveTick`
  (params (DeltaSeconds :type "Float (single-precision)"))
  (set `self.CurrentTime` (+ DeltaSeconds (`self.CurrentTime`)))
  (`LightComponent.SetIntensity` (`self.PointLight`) (- (`LightComponentBase.Intensity` (`self.PointLight`)) (`self.DecreaseScale`)))
  (if (>= (`self.CurrentTime`) (`self.DestroyTime`))
    (`self.K2_DestroyActor`)))

(event `self.ReceiveActorBeginOverlap`
  (params (OtherActor :type "Actor Object Reference"))
  (bind _asbase_enemy (cast `BaseEnemy` OtherActor))
  (cast `Character` (`self.Instigator`))
  (`BaseEnemy.GetDamage` _asbase_enemy (make `GenericAttackParams` null (`self.Damage`) (`self.StunDamage`) "DOWN" true)))

(fn `UserConstructionScript`)